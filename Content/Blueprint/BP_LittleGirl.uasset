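; BP_LittleGirl is a little girl pawn that walks a route of destinations while carrying an item.
; StarttoWalk copies the placeable model from a BP_PickupPictures actor onto EquipedItem, then, if State allows, starts AIMoveTo toward the current Destinations entry.
; Each successful move advances Target and loops to the next entry; the last resets Target and destroys the carried item.
; Failed moves are not handled.
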(event `self.ReceiveBeginPlay`)

(event `StarttoWalk`
  (bind _returnvalue (+ (`self.Target`) 1))
  (bind _returnvalue_2 (`GameplayStatics.GetActorOfClass` "/Game/Blueprint/BP_PickupPictures.BP_PickupPictures_C"))
  (`StaticMeshComponent.SetStaticMesh` (`self.EquipedItem`) (`/Game/Blueprint/BP_PickupPictures.ItemModelToPlace` _returnvalue_2))
  (if (`|EnumEquality` (`self.State`) "NewEnumerator0")
    (`|AIMoveTo` self (0.0 0.0 0.0) (`|GetArrayItem` (`self.Destinations`) (`self.Target`)) :!label _label
      (:`OnSuccess`
        (if (== (`KismetArrayLibrary.Array_Length` (`self.Destinations`)) _returnvalue)
          (set `self.Target` 0)
          (`ActorComponent.K2_DestroyComponent` (`self.EquipedItem`))
          (else
            (set `self.Target` _returnvalue)
            (goto _label)))))))

(fn `UserConstructionScript`)